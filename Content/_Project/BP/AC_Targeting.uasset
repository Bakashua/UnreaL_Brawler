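; Actor component that gives its owning Character a toggleable lock-on to nearby Pawns.
; Targeting sphere-traces along the camera's forward vector and picks the hit actor whose direction best matches it by dot product.
; While locked, Tick aims control rotation at the target, switches movement from orient-to-movement to controller-driven rotation, and shortens and lowers the spring arm at close range.
; Debug prints and trace drawing are active.
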(event `self.ReceiveBeginPlay`
  (bind _returnvalue (`self.GetOwner`))
  (set `self.PlayerCam` (`Actor.GetComponentByClass` _returnvalue "/Script/Engine.CameraComponent"))
  (set `self.PlayerSpringArm` (`Actor.GetComponentByClass` _returnvalue "/Script/Engine.SpringArmComponent"))
  (set `self.PlayerMovementComponent` (`Actor.GetComponentByClass` _returnvalue "/Script/Engine.CharacterMovementComponent"))
  (bind _ascharacter (cast `Character` (`self.GetOwner`)))
  (set `self.OwnerCharacter` _ascharacter))

(event `self.ReceiveTick`
  (params (DeltaSeconds :type "Float (single-precision)"))
  (bind _currenttarget (`self.CurrentTarget`))
  (bind _playerspringarm (`self.PlayerSpringArm`))
  (`|ExecutionSequence`
    (:`then_0`
      (`self.CurrentTarget`
        (:`then`
          (`KismetSystemLibrary.PrintString` (`KismetStringLibrary.Conv_RotatorToString` (`SceneComponent.K2_GetComponentRotation` (`self.PlayerCam`))) true true (struct :`R` 0.981331 :`G` 1.0 :`B` 0.673907 :`A` 1.0) 2.0 "Nonie")
          (if (<= (`KismetMathLibrary.Vector_Distance` (`Actor.K2_GetActorLocation` (`self.CurrentTarget`)) (`SceneComponent.K2_GetComponentLocation` (`Actor.RootComponent` (`self.OwnerCharacter`)))) 300.0)
            (set `SpringArmComponent.TargetArmLength` 200.0 _playerspringarm)
            (set `SpringArmComponent.SocketOffset` (`KismetMathLibrary.MakeVector` 0.0 0.0 (`KismetMathLibrary.Lerp` 50.0 20.0 (`GameplayStatics.GetWorldDeltaSeconds`))) _playerspringarm)
            (else
              (set `SpringArmComponent.TargetArmLength` 300.0 _playerspringarm)
              (set `SpringArmComponent.SocketOffset` (0.0 0.0 50.0) _playerspringarm))))
        (:`else`)))
    (:`then_1`
      (`self.CurrentTarget`
        (:`then`
          (bind _playermovementcomponent (`self.PlayerMovementComponent`)
            (:`then`
              (set `CharacterMovementComponent.bOrientRotationToMovement` false _playermovementcomponent)
              (set `CharacterMovementComponent.bUseControllerDesiredRotation` true _playermovementcomponent)
              (`Controller.SetControlRotation` (`Pawn.GetController` (`self.OwnerCharacter`)) (`KismetMathLibrary.FindLookAtRotation` (`SceneComponent.K2_GetComponentLocation` (`self.PlayerCam`)) (`Actor.K2_GetActorLocation` _currenttarget)))
              (`KismetSystemLibrary.PrintString` (`KismetSystemLibrary.GetDisplayName` _currenttarget) true true (struct :`G` 0.66 :`B` 1.0 :`A` 1.0) 2.0 "rrNone"))
            (:`else`)))
        (:`else`
          (bind _playermovementcomponent_2 (`self.PlayerMovementComponent`)
            (:`then`
              (set `CharacterMovementComponent.bOrientRotationToMovement` true _playermovementcomponent_2)
              (set `CharacterMovementComponent.bUseControllerDesiredRotation` false _playermovementcomponent_2))
            (:`else`)))))))

(event `EVT_ToggleTargeting`
  (`self.CurrentTarget`
    (:`then`
      (`self.EVT_Untarget`))
    (:`else`
      (`self.EVT_TryFindTarget`))))

(event `EVT_TryFindTarget`
  (bind (_found _foundtarget) (`self.FindTarget`))
  (if _found
    (set `self.CurrentTarget` _foundtarget)))

(event `EVT_Untarget`
  (set `self.CurrentTarget` null))

(fn `FaceTargetDirection`
  (`self.EVT_ToggleTargeting`))

(fn `FindTarget`
  (returns (Found :type Boolean) (FoundTarget :type "Actor Object Reference"))
  (bind _returnvalue (`self.GetOwner`))
  (bind _returnvalue_2 (`Actor.K2_GetActorLocation` _returnvalue))
  (bind (_outhits _returnvalue_3) (`KismetSystemLibrary.SphereTraceMultiForObjects` _returnvalue_2 (+ _returnvalue_2 (* (`SceneComponent.GetForwardVector` (`self.PlayerCam`)) 1000.0)) 0.0 (`|MakeArray` "ObjectTypeQuery3" :!type "EObjectTypeQuery Enum") false (`|MakeArray` _returnvalue) "ForOneFrame"))
  (if _returnvalue_3
    (for _array_element _outhits
      (`KismetArrayLibrary.Array_AddUnique` (`self.PotentialTarget`) (`.HitActor` (`GameplayStatics.BreakHitResult` _array_element))))
    (bind (_found _foundtarget) (`self.GetBestTarget` (`self.PotentialTarget`)))
    (return _found _foundtarget)))

(fn `GetBestTarget`
  (params (PotentialTarget :type "Array of Actor Object Reference"))
  (returns (Found :type Boolean) (FoundTarget :type "Actor Object Reference"))
  (locals (Dots :type "Array of Float (double-precision)"))
  (bind _output (`|GetArrayItem` PotentialTarget (`KismetMathLibrary.MaxOfFloatArray` (`local.Dots`))))
  (for _array_element PotentialTarget
    (`KismetArrayLibrary.Array_Add` (`local.Dots`) (`KismetMathLibrary.Dot_VectorVector` (`KismetMathLibrary.Normal` (- (`Actor.K2_GetActorLocation` _array_element) (`Actor.K2_GetActorLocation` (`self.GetOwner`)))) (`SceneComponent.GetForwardVector` (`self.PlayerCam`)))))
  (return (`KismetSystemLibrary.IsValid` _output) _output))